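; Floor tile for a runner game that spawns an obstacle on itself and cleans up after the player passes.
; On BeginPlay it spawns an obstacle using a random ObstaclePositions entry, offset by the tile's location, and stores a reference to it.
; The first ThirdPersonCharacter overlap with its Collision starts a delay, after which it destroys both obstacle and tile.
; A score addition through the runner game mode is left unconnected.
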(event OnComponentBeginOverlap(Collision)
  (params (OverlappedComponent :type Primitive%20Component%20Object%20Reference) (OtherActor :type Actor%20Object%20Reference) (OtherComp :type Primitive%20Component%20Object%20Reference) (OtherBodyIndex :type Integer) (bFromSweep :type Boolean) (SweepResult :type Hit%20Result%20Structure%20%28by%20ref%29))
  (Utilities|Casting|CastToThirdPersonCharacter OtherActor)
  (if (not (Variables|Default|GetbPlayerPassed))
    (Variables|Default|SetbPlayerPassed true)
    (Utilities|FlowControl|Delay 1e+01)
    (Actor|DestroyActor (Variables|Default|GetObstacleReference))
    (Actor|DestroyActor)))

(event EventBeginPlay
  (bind _obstaclepositions (Variables|Default|GetObstaclePositions))
  (bind _returnvalue (Utilities|Array|Length _obstaclepositions))
  (bind _returnvalue_2 (- _returnvalue 1))
  (bind _returnvalue_3 (Math|Random|RandomIntegerinRange 0 _returnvalue_2))
  (bind _output (Utilities|Array|Get(acopy) _obstaclepositions _returnvalue_3))
  ;[1 1 1] Spawn obstacle from positions list
  (bind _returnvalue_4 (Game|SpawnActorfromClass "/Game/Blueprints/BP_Obstacle.BP_Obstacle_C" (Math|Transform|MakeTransform (+ (.location _output) (.location (Transformation|GetActorTransform))) (.rotation _output) (.scale _output)) "Undefined" 0 0))
  (Variables|Default|SetObstacleReference _returnvalue_4))

(fn ConstructionScript)