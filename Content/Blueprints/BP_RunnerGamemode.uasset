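; BP_RunnerGamemode is the runner game mode that keeps extending the floor by spawning BP_FloorTile actors.
; BeginPlay caches a placed tile as FrontTile and starts a looping one-second timer.
; Each tick of that timer spawns one tile at FrontTile's TileMarker, keeping its rotation and scale, if the live tile count is below TileLimit.
; The new tile becomes FrontTile, chaining the track forward.
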(event Custom|TileGeneration
  (bind _outactors (Actor|GetAllActorsOfClass "/Game/Blueprints/BP_FloorTile.BP_FloorTile_C"))
  (if (< (Utilities|Array|Length _outactors) (Variables|Default|GetTileLimit)) ; If tile limit has not been reached
    (bind _returnvalue (Game|SpawnActorfromClass "/Game/Blueprints/BP_FloorTile.BP_FloorTile_C" (Math|Transform|MakeTransform (Transformation|GetWorldLocation (Variables|/Game/Blueprints/BP_FloorTile.BP_FloorTile_C|GetTileMarker (Variables|Default|GetFrontTile))) (.rotation (Transformation|GetActorTransform (Variables|Default|GetFrontTile))) (.scale (Transformation|GetActorTransform (Variables|Default|GetFrontTile)))) "Undefined" 0 0))
    (Variables|Default|SetFrontTile _returnvalue)))

(event EventBeginPlay
  ;[1 1 1] Save first tile
  (bind _returnvalue (Actor|GetActorOfClass "/Game/Blueprints/BP_FloorTile.BP_FloorTile_C"))
  (Variables|Default|SetFrontTile _returnvalue)
  (Utilities|Time|SetTimerbyEvent (delegate Custom|TileGeneration) 1.0 true))

(fn ConstructionScript)